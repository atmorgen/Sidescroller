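; BP_Triplets is a flip platform with a Paper2D sprite that toggles between solid and passable when its Flip event fires.
; Flip tints the sprite white or black from IsFlipped, switches collision between none and query-and-physics based on its current state, then inverts the flag.
; An older visibility-toggle variant remains in the graph, unconnected.
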(event `Flip`
  (bind _papersprite (`self.PaperSprite`))
  (bind _papersprite_2 (`self.PaperSprite`))
  (if (`self.isFlipped`)
    (`PaperSpriteComponent.SetSpriteColor` _papersprite (`KismetMathLibrary.LinearColor_White`))
    (else
      (`PaperSpriteComponent.SetSpriteColor` _papersprite (`KismetMathLibrary.LinearColor_Black`))))
  (switch `ECollisionEnabled` (`PrimitiveComponent.GetCollisionEnabled` (`self.PaperSprite`))
    (:`NoCollision`
      (`PrimitiveComponent.SetCollisionEnabled` _papersprite_2 "QueryAndPhysics"))
    (:`QueryAndPhysics`
      (`PrimitiveComponent.SetCollisionEnabled` _papersprite_2 "NoCollision")))
  (set `self.isFlipped` (not (`self.isFlipped`))))

(fn `UserConstructionScript`)