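; Trampoline platform that launches BP_SprintCharacter on overlap with its box, using a stronger velocity while the timing flag is set.
; RunTrampLogic starts two parallel delayed events: one toggles IsCorrectTime at both ends of BoostWindow, the other refreshes the sprite tint alongside it.
; The sprite shows white for correct timing and red otherwise, and launches override the character's existing velocity.
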(event `RunTrampLogic`
  (`self.CorrectTiming`)
  (`self.SetVisualsTiming`))

(event `CorrectTiming`
  (`self.SetIsCorrectTiming`)
  (`KismetSystemLibrary.Delay` (`self.boostWindow`))
  (`self.SetIsCorrectTiming`))

(event `SetIsCorrectTiming`
  (set `self.isCorrectTime` (not (`self.isCorrectTime`))))

(event `SetVisualsTiming`
  (`self.SetVisuals`)
  (`KismetSystemLibrary.Delay` (`self.boostWindow`))
  (`self.SetVisuals`))

(event `SetVisuals`
  (if (`self.isCorrectTime`)
    (`PaperSpriteComponent.SetSpriteColor` (`self.PaperSprite`) (`KismetMathLibrary.LinearColor_White`))
    (else
      (`PaperSpriteComponent.SetSpriteColor` (`self.PaperSprite`) (`KismetMathLibrary.LinearColor_Red`)))))

(event `self.Box.OnComponentBeginOverlap`
  (params (OverlappedComponent :type "PrimitiveComponent Object Reference") (OtherActor :type "Actor Object Reference") (OtherComp :type "PrimitiveComponent Object Reference") (OtherBodyIndex :type Integer) (bFromSweep :type Boolean) (SweepResult :type "HitResult Structure (by ref)"))
  (bind _asbp_sprint_character (cast `/Game/Blueprints/BP_SprintCharacter` OtherActor))
  (if (`self.isCorrectTime`)
    (`Character.LaunchCharacter` _asbp_sprint_character (`self.TrampValueMax`) true true)
    (else
      (`Character.LaunchCharacter` _asbp_sprint_character (`self.TrampValueMin`) true true))))

(fn `UserConstructionScript`)