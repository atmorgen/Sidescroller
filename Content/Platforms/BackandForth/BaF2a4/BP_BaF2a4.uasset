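; Paper2D platform Blueprint that slides its sprite back and forth along its local X axis.
; Every Tick calls BackandForth, which offsets the sprite one unit per frame without sweeping, in the direction set by GoingForward.
; Movement is not scaled by delta time, so speed depends on frame rate.
; Switch_goingForward flips the direction and is not called within this Blueprint.
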(event `self.ReceiveTick`
  (params (DeltaSeconds :type "Float (single-precision)"))
  (`self.BackandForth`))

(event `BackandForth`
  (bind _papersprite (`self.PaperSprite`))
  (if (`self.goingForward`)
    (`SceneComponent.K2_AddLocalOffset` _papersprite (1.0 0.0 0.0) false false)
    (else
      (`SceneComponent.K2_AddLocalOffset` _papersprite (-1.0 0.0 0.0) false false))))

(event `Switch_goingForward`
  (set `self.goingForward` (not (`self.goingForward`))))

(fn `UserConstructionScript`)